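; Player pawn that turns input into rotation of the level's Temple and spawning of a Ball.
; The RotateTemple axis accumulates an inverted value, which is scaled and applied as the yaw of the Temple actor.
; Pressing LaunchBall spawns a Ball just above the first Launcher, only when no other Ball exists in the level.
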(event Input|ActionEvents|InputActionLaunchBall
  (params (Key :type Key%20Structure :default "None"))
  (:Pressed
    (bind _outactors (Actor|GetAllActorsOfClass "/Game/Blueprints/Launcher.Launcher_C"))
    (bind _outactors_2 (Actor|GetAllActorsOfClass "/Game/Blueprints/Ball.Ball_C"))
    (if (== (Utilities|Array|Length _outactors_2) 0)
      (Game|SpawnActorfromClass "/Game/Blueprints/Ball.Ball_C" (Math|Transform|MakeTransform (Math|Vector|MakeVector (.X (Math|Vector|BreakVector (Transformation|GetActorLocation (Utilities|Array|Get(acopy) _outactors)))) (.Y (Math|Vector|BreakVector (Transformation|GetActorLocation (Utilities|Array|Get(acopy) _outactors)))) (+ (.Z (Math|Vector|BreakVector (Transformation|GetActorLocation (Utilities|Array|Get(acopy) _outactors)))) 1e+01))) "Undefined" 0 0))))

(event Input|AxisEvents|InputAxisRotateTemple
  (params (AxisValue :type Float%20%28single-precision%29))
  (bind _output_get (Variables|Default|SetRotateValue (+ (* AxisValue -1.0) (Variables|Default|GetRotateValue))))
  (bind _returnvalue (Actor|GetActorOfClass "/Game/Blueprints/Temple.Temple_C"))
  (Transformation|SetActorRotation _returnvalue (Math|Rotator|MakeRotator 0.0 0.0 (* _output_get 2.0))))

(fn ConstructionScript)